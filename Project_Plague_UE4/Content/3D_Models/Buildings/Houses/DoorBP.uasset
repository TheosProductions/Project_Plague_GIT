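; Interactive house door Blueprint that the player swings open and closed with the OpenDoor input.
; A box trigger enables the door's input on overlap and disables it when the overlap ends.
; Each press flips DoorIsOpen and plays or reverses the DoorRotation timeline, which drives the DoorPivot yaw.
; The FirstPersonCharacter's Mesh2P plays the door-opening animation both ways, returning to Animation Blueprint mode when the timeline finishes.
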(event `self.Box.OnComponentBeginOverlap`
  (params (OverlappedComponent :type "PrimitiveComponent Object Reference") (OtherActor :type "Actor Object Reference") (OtherComp :type "PrimitiveComponent Object Reference") (OtherBodyIndex :type Integer) (bFromSweep :type Boolean) (SweepResult :type "HitResult Structure (by ref)"))
  ;[1 1 1] Enable/Disable Input
  (`self.EnableInput` (`GameplayStatics.GetPlayerController` 0)))

(event `self.Box.OnComponentEndOverlap`
  (params (OverlappedComponent :type "PrimitiveComponent Object Reference") (OtherActor :type "Actor Object Reference") (OtherComp :type "PrimitiveComponent Object Reference") (OtherBodyIndex :type Integer))
  ;[1 1 1] Enable/Disable Input
  (`self.DisableInput` (`GameplayStatics.GetPlayerController` 0)))

(event `InputAction|OpenDoor`
  (params (Key :type "Key Structure"))
  (bind _returnvalue (`GameplayStatics.GetPlayerCharacter` 0))
  (:`Pressed`
    (if (`self.DoorIsOpen`)
      (set `self.DoorIsOpen` false)
      (bind _asfirst_person_character (cast `/Game/FirstPersonBP/Blueprints/FirstPersonCharacter` _returnvalue))
      (`SkeletalMeshComponent.PlayAnimation` (`/Game/FirstPersonBP/Blueprints/FirstPersonCharacter.Mesh2P` _asfirst_person_character) "/Game/FirstPerson/Animations/Player/OPENING_DOOR_Anim.OPENING_DOOR_Anim" false)
      (bind (_direction _doorrotation) (`Timeline|DoorRotation` :!label _label)
        (:`Update`
          (`SceneComponent.K2_SetRelativeRotation` (`self.Door Pivot`) (`KismetMathLibrary.MakeRotator` 0.0 0.0 _doorrotation) false false))
        (:`Finished`
          (bind _asfirst_person_character_2 (cast `/Game/FirstPersonBP/Blueprints/FirstPersonCharacter` (`GameplayStatics.GetPlayerCharacter` 0)))
          (`SkeletalMeshComponent.SetAnimationMode` (`/Game/FirstPersonBP/Blueprints/FirstPersonCharacter.Mesh2P` _asfirst_person_character_2) "AnimationBlueprint")))
      (else
        (set `self.DoorIsOpen` true)
        (bind _asfirst_person_character_3 (cast `/Game/FirstPersonBP/Blueprints/FirstPersonCharacter` _returnvalue))
        (`SkeletalMeshComponent.PlayAnimation` (`/Game/FirstPersonBP/Blueprints/FirstPersonCharacter.Mesh2P` _asfirst_person_character_3) "/Game/FirstPerson/Animations/Player/OPENING_DOOR_Anim.OPENING_DOOR_Anim" false)
        (goto _label :!via `Reverse`)))))

(fn `UserConstructionScript`)